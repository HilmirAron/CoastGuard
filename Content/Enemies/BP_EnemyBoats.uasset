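; Enemy boat on a tile board that shows a countdown, facing the camera, and acts when CountDown brings it to zero.
; Its action moves it onto an orthogonal neighbour tile holding the player, otherwise to a random neighbour without island or enemy boat, using a timeline lerp.
; Overlapping the player calls ShipDead and destroys the boat, while Death spawns an explosion and a nuke fuel pickup.
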(event `self.ReceiveBeginPlay`
  ;[1 1 1] Begin Play, set text and find player
  (set `self.MyCount` (`self.startingCount`))
  (`TextRenderComponent.K2_SetText` (`self.TextRender`) (`KismetTextLibrary.Conv_IntToText` (`self.MyCount`)))
  (bind _returnvalue (`GameplayStatics.GetActorOfClass` "/Game/BLueprints/BP_Character.BP_Character_C"))
  (set `self.PlayerRef` _returnvalue))

(event `self.ReceiveTick`
  (params (DeltaSeconds :type "Float (single-precision)"))
  (`SceneComponent.K2_SetWorldRotation` (`self.TextRender`) (`KismetMathLibrary.FindLookAtRotation` (`SceneComponent.K2_GetComponentLocation` (`self.TextRender`)) (`self.K2_GetActorLocation` (`GameplayStatics.GetPlayerCameraManager` 0))) false false))

(event `CountDown`
  (bind _result (`/Engine/EditorBlueprintResources/StandardMacros.DecrementInt` (`self.MyCount`))
    (:`  `
      (if (== _result 0)
        (`self.DoAction`)
        (set `self.MyCount` (`self.startingCount`))
        (`TextRenderComponent.K2_SetText` (`self.TextRender`) (`KismetTextLibrary.Conv_IntToText` (`self.MyCount`)))
        (else
          (`TextRenderComponent.K2_SetText` (`self.TextRender`) (`KismetTextLibrary.Conv_IntToText` (`self.MyCount`))))))))

(event `DoAction`
  (bind _neighbours (`self.GetNeighbours`))
  (for _array_element _neighbours
    (bind _output (`/Game/BLueprints/BP_Comp_Tile.GetActorOnTile` _array_element))
    (cast `/Game/BLueprints/BP_Character` _output)
    (`self.MoveBoat` _array_element)
    (set `self.destroyed` true))
  (if (not (`self.destroyed`))
    (bind _newparam (`self.Randomtile`))
    (`self.MoveBoat` _newparam)))

(event `self.StaticMesh.OnComponentBeginOverlap`
  (params (OverlappedComponent :type "PrimitiveComponent Object Reference") (OtherActor :type "Actor Object Reference") (OtherComp :type "PrimitiveComponent Object Reference") (OtherBodyIndex :type Integer) (bFromSweep :type Boolean) (SweepResult :type "HitResult Structure (by ref)"))
  (bind _asbp_character (cast `/Game/BLueprints/BP_Character` OtherActor))
  (`/Game/BLueprints/BP_Character.ShipDead` _asbp_character)
  (`self.K2_DestroyActor`))

(event `StartMoving`
  (params (Beginning :type "Vector Structure") (End :type "Vector Structure"))
  (bind (_direction _newtrack_0) (`Timeline|Movement` :!via `PlayFromStart`)
    (:`Update`
      (`self.K2_SetActorLocation` (`KismetMathLibrary.VLerp` Beginning End _newtrack_0)))))

(event `Death`
  (`GameplayStatics.SpawnEmitterAtLocation` "/Game/Realistic_Starter_VFX_Pack_Vol2/Particles/Explosion/P_Explosion_Big_C.P_Explosion_Big_C" (`self.K2_GetActorLocation`) (struct) (0.3 0.3 0.3))
  (if (`KismetMathLibrary.RandomBoolWithWeight` 1.0)
    (`|SpawnActorFromClass` "/Game/BP_NukeFuel.BP_NukeFuel_C" (`KismetMathLibrary.MakeTransform` (+ (`self.K2_GetActorLocation`) (0.0 0.0 50.0))) "Undefined" "MultiplyWithRoot" null null))
  (`self.K2_DestroyActor`))

(fn `GetNeighbours`
  (returns (Neighbours :type "Array of /Game/BLueprints/BP_Comp_Tile Object Reference"))
  (locals (neighboursTiles :type "Array of /Game/BLueprints/BP_Comp_Tile Object Reference"))
  (bind (_enemycurrenttile_x _enemycurrenttile_y) (`KismetMathLibrary.BreakVector2D` (`self.EnemyCurrentTile`)))
  (bind (_enemycurrenttile_x_2 _enemycurrenttile_y_2) (`KismetMathLibrary.BreakVector2D` (`self.EnemyCurrentTile`)))
  (bind (_enemycurrenttile_x_3 _enemycurrenttile_y_3) (`KismetMathLibrary.BreakVector2D` (`self.EnemyCurrentTile`)))
  (bind (_enemycurrenttile_x_4 _enemycurrenttile_y_4) (`KismetMathLibrary.BreakVector2D` (`self.EnemyCurrentTile`)))
  (bind _tile (`/Game/BLueprints/bp_tileboard.FindTile` (`/Game/BLueprints/BP_Character.tileBoardRef` (`self.PlayerRef`)) (`KismetMathLibrary.MakeVector2D` (+ _enemycurrenttile_x_3 1.0) (+ _enemycurrenttile_y_3 0.0))))
  (`/Engine/EditorBlueprintResources/StandardMacros.IsValid` _tile
    (:`Is Valid`
      (`KismetArrayLibrary.Array_Add` (`local.neighboursTiles`) _tile))
    (:`Is Not Valid`
      _))
  (bind _tile_2 (`/Game/BLueprints/bp_tileboard.FindTile` (`/Game/BLueprints/BP_Character.tileBoardRef` (`self.PlayerRef`)) (`KismetMathLibrary.MakeVector2D` (+ _enemycurrenttile_x_4 -1.0) (+ _enemycurrenttile_y_4 0.0))))
  (`/Engine/EditorBlueprintResources/StandardMacros.IsValid` _tile_2
    (:`Is Valid`
      (`KismetArrayLibrary.Array_Add` (`local.neighboursTiles`) _tile_2))
    (:`Is Not Valid`
      _))
  (bind _tile_3 (`/Game/BLueprints/bp_tileboard.FindTile` (`/Game/BLueprints/BP_Character.tileBoardRef` (`self.PlayerRef`)) (`KismetMathLibrary.MakeVector2D` (+ _enemycurrenttile_x_2 0.0) (+ _enemycurrenttile_y_2 1.0))))
  (`/Engine/EditorBlueprintResources/StandardMacros.IsValid` _tile_3
    (:`Is Valid`
      (`KismetArrayLibrary.Array_Add` (`local.neighboursTiles`) _tile_3))
    (:`Is Not Valid`
      _))
  (bind _tile_4 (`/Game/BLueprints/bp_tileboard.FindTile` (`/Game/BLueprints/BP_Character.tileBoardRef` (`self.PlayerRef`)) (`KismetMathLibrary.MakeVector2D` (+ _enemycurrenttile_x 0.0) (+ _enemycurrenttile_y -1.0))))
  (`/Engine/EditorBlueprintResources/StandardMacros.IsValid` _tile_4
    (:`Is Valid`
      (`KismetArrayLibrary.Array_Add` (`local.neighboursTiles`) _tile_4))
    (:`Is Not Valid`
      _))
  (return (`local.neighboursTiles`)))

(fn `MoveBoat`
  (params (Tile :type "/Game/BLueprints/BP_Comp_Tile Object Reference"))
  (bind _myid (`/Game/BLueprints/BP_Comp_Tile.MyID` Tile))
  (bind (_returnvalue_x _returnvalue_y) (`KismetMathLibrary.BreakVector2D` (- _myid (`self.EnemyCurrentTile`))))
  (`self.StartMoving` (`self.K2_GetActorLocation`) (`SceneComponent.K2_GetComponentLocation` Tile))
  (`self.K2_SetActorRotation` (`KismetMathLibrary.MakeRotator` 0.0 0.0 (+ (`KismetMathLibrary.SelectFloat` 180.0 0.0 (< _returnvalue_x 0.0)) (* _returnvalue_y -90.0))))
  (set `self.EnemyCurrentTile` _myid))

(fn `Randomtile`
  (returns (NewParam :type "/Game/BLueprints/BP_Comp_Tile Object Reference"))
  (locals (SafeTiles :type "Array of /Game/BLueprints/BP_Comp_Tile Object Reference"))
  (bind _neighbours (`self.GetNeighbours`))
  (for _array_element _neighbours
    (if (not (`/Game/BLueprints/BP_Comp_Tile.IsIsland` _array_element))
      (bind _output (`/Game/BLueprints/BP_Comp_Tile.GetActorOnTile` _array_element))
      (cast `/Game/Enemies/BP_EnemyBoats` _output
        (:`CastFailed`
          (`KismetArrayLibrary.Array_Add` (`local.SafeTiles`) _array_element)))))
  (return (`KismetArrayLibrary.Array_Random` (`local.SafeTiles`))))

(fn `UserConstructionScript`)