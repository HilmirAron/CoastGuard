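; Enemy cannon Blueprint that fires from both sides, port and starboard.
; On DoAction, it loops over the Starboard and Port components and spawns a Bp_cannons actor at each world transform.
; Each spawned actor receives this Blueprint as Maker and has EnemyBall set to true.
; The event holds all the logic, as BeginPlay, overlap and Tick are disabled stubs.
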(event `self.DoAction`
  (for _array_element (`|MakeArray` (`self.Starboard`) (`self.Port`))
    (`|SpawnActorFromClass` "/Game/BLueprints/bp_cannons.bp_cannons_C" (`SceneComponent.K2_GetComponentToWorld` _array_element) "Undefined" "MultiplyWithRoot" null self true null)))

(fn `UserConstructionScript`
  (`parent.UserConstructionScript`))