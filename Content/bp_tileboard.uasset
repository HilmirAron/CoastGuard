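; Tile board actor that builds a square grid of tile components and populates its ocean with enemy boats at the start of a level.
; Construction assigns each tile a grid ID for FindTile lookups, and FindAllOcean filters out islands.
; BeginPlay randomly seeds boats on ocean tiles, guarantees at least one, then has the character reference spawn the player.
; EnemyKilled opens Map_Fusion once no boats remain.
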(event `self.ReceiveBeginPlay`
  (bind _newparam (`self.FindAllOcean`))
  (for _array_element _newparam
    (if (`KismetMathLibrary.RandomBoolWithWeight` 0.1)
      (`|SpawnActorFromClass` "/Game/BP_EnemyBoats.BP_EnemyBoats_C" (`KismetMathLibrary.MakeTransform` (`SceneComponent.K2_GetComponentLocation` _array_element) (`KismetMathLibrary.MakeRotator` 0.0 0.0 (select `int` (`KismetMathLibrary.RandomInteger` 3) :`0` 0.0 :`1` 90.0 :`2` 180.0 :`3` 270.0 :!type "Float (single-precision)"))) "Undefined" "MultiplyWithRoot" null (`/Game/BP_Comp_Tile.MyID` _array_element) null)
      (`KismetArrayLibrary.Array_Add` (`self.tileWithEnemies`) _array_element)))
  (bind _outactors (`GameplayStatics.GetAllActorsOfClass` "/Game/BP_EnemyBoats.BP_EnemyBoats_C"))
  (if (> (`KismetArrayLibrary.Array_Length` _outactors) 0)
    (`/Game/BP_Character.SpawnPalyer` (`self.CharacterREf`))
    (else
      (bind _newparam_2 (`self.FindAllOcean`))
      (bind _output_get (set `self.RandomTile` (`KismetArrayLibrary.Array_Random` _newparam_2)))
      (`|SpawnActorFromClass` "/Game/BP_EnemyBoats.BP_EnemyBoats_C" (`KismetMathLibrary.MakeTransform` (`SceneComponent.K2_GetComponentLocation` _output_get) (`KismetMathLibrary.MakeRotator` 0.0 0.0 (select `int` (`KismetMathLibrary.RandomInteger` 3) :`0` 0.0 :`1` 90.0 :`2` 180.0 :`3` 270.0 :!type "Float (single-precision)"))) "Undefined" "MultiplyWithRoot" null (`/Game/BP_Comp_Tile.MyID` _output_get) null)
      (`KismetArrayLibrary.Array_Add` (`self.tileWithEnemies`) (`self.RandomTile`))
      (`/Game/BP_Character.SpawnPalyer` (`self.CharacterREf`)))))

(event `EnemyKilled`
  (bind _outactors (`GameplayStatics.GetAllActorsOfClass` "/Game/BP_EnemyBoats.BP_EnemyBoats_C"))
  (if (not (> (`KismetArrayLibrary.Array_Length` _outactors) 0))
    (`GameplayStatics.OpenLevel` "Map_Fusion")))

(fn `FindAllOcean`
  (returns (NewParam :type "Array of /Game/BP_Comp_Tile Object Reference"))
  (locals (FoundOcean :type "Array of /Game/BP_Comp_Tile Object Reference"))
  (for _array_element (`self.K2_GetComponentsByClass` "/Game/BP_Comp_Tile.BP_Comp_Tile_C")
    (if (not (`/Game/BP_Comp_Tile.IsIsland` _array_element))
      (`KismetArrayLibrary.Array_Add` (`local.FoundOcean`) _array_element)))
  (return (`local.FoundOcean`)))

(fn `FindTile`
  (params (ID :type "Vector2D Structure"))
  (returns (TIle :type "/Game/BP_Comp_Tile Object Reference"))
  (locals (FoundTiles1 :type "Array of /Game/BP_Comp_Tile Object Reference") (FoundTiles2 :type "Array of /Game/BP_Comp_Tile Object Reference"))
  (for _array_element (`self.K2_GetComponentsByClass` "/Game/BP_Comp_Tile.BP_Comp_Tile_C")
    (if (`KismetMathLibrary.EqualExactly_Vector2DVector2D` (`/Game/BP_Comp_Tile.MyID` _array_element) ID)
      (return _array_element))))

(fn `UserConstructionScript`
  (bind _space (`self.Space`))
  (bind _returnvalue (- (`self.TileSize`) 1))
  (for _index (range (+ _returnvalue 1))
    (for _index_2 (range (+ _returnvalue 1))
      (bind _returnvalue_2 (`AddComponent|NODE_AddBP_Comp_Tile-0` :`RelativeTransform` (`KismetMathLibrary.MakeTransform` (`KismetMathLibrary.MakeVector` (* _index _space) (* _index_2 _space)))))
      (set `/Game/BP_Comp_Tile.MyID` (`KismetMathLibrary.MakeVector2D` (`KismetMathLibrary.Conv_IntToDouble` _index_2) (`KismetMathLibrary.Conv_IntToDouble` _index)) _returnvalue_2))))