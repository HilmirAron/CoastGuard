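; Tile component that randomly becomes an island and can report the actor standing on it.
; On BeginPlay it has a 5% chance to switch to the island material and set its island flag.
; It also binds a cursor-over event that prints the tile's ID, and GetActorOnTile returns the first overlapping actor without checking that one exists.
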(event `self.ReceiveBeginPlay`
  (add `self.OnBeginCursorOver` (delegate `CustomEvent`))
  (if (`KismetMathLibrary.RandomBoolWithWeight` 0.05)
    (`self.SetMaterial` 0 "/Game/materials/Mat_Island.Mat_Island")
    (set `self.IsIsland` true)))

(event `CustomEvent` :!signature `self.OnBeginCursorOver`
  (params (TouchedComponent :type "PrimitiveComponent Object Reference"))
  (`KismetSystemLibrary.PrintString` (`KismetStringLibrary.Conv_Vector2dToString` (`self.MyID`))))

(fn `GetActorOnTile`
  (returns (Output :type "Actor Object Reference"))
  (return (`|GetArrayItem` (`self.GetOverlappingActors` null))))