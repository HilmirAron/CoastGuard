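; BP_Character is the player's ship in a turn-based, tile-board naval game.
; It spawns on a random tile free of islands and enemies, then steps between tiles with Enhanced Input, turning its mesh and staying off islands.
; Space fires cannons from port and starboard, blocking actions briefly.
; Each completed move or volley counts down every enemy boat; death shows the death widget and destroys the ship.
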(event `SpawnPalyer`
  ;[1 1 1] Select a random Tile and spawn there
  (bind _out (`self.SafePlace`))
  (bind _output_get (set `self.CurrentTile` (`/Game/BLueprints/BP_Comp_Tile.MyID` (`KismetArrayLibrary.Array_Random` _out))))
  (bind _tile (`/Game/BLueprints/bp_tileboard.FindTile` (`self.tileBoardRef`) _output_get))
  (`self.K2_SetActorLocation` (`SceneComponent.K2_GetComponentLocation` _tile)))

(event `self.ReceiveBeginPlay`
  (bind _returnvalue (`GameplayStatics.GetPlayerController` 0))
  (bind _returnvalue_2 (pcsubsystem `EnhancedInputLocalPlayerSubsystem` _returnvalue))
  ;[1 1 1] Set up input
  (`self.EnableInput` _returnvalue)
  (`/Engine/EditorBlueprintResources/StandardMacros.IsValid` _returnvalue_2
    (:`Is Valid`
      (message `EnhancedInputSubsystemInterface.AddMappingContext` _returnvalue_2 "/Game/Input/IMC_Player.IMC_Player" 0 (struct))
      (set `PlayerController.bEnableMouseOverEvents` true (`GameplayStatics.GetPlayerController` 0)))))

(event `ActionDone`
  (bind _outactors (`GameplayStatics.GetAllActorsOfClass` "/Game/Enemies/BP_EnemyBoats.BP_EnemyBoats_C"))
  (for _array_element _outactors
    (`/Game/Enemies/BP_EnemyBoats.CountDown` _array_element)))

(event `EnhancedInput|/Game/Input/IA_Move`
  (params (ActionValue :type "Vector2D Structure") (ElapsedSeconds :type "Float (double-precision)") (TriggeredSeconds :type "Float (double-precision)") (InputAction :type "InputAction Object Reference" :default "/Game/Input/IA_Move.IA_Move"))
  (bind (_currenttile_x _currenttile_y) (`KismetMathLibrary.BreakVector2D` (`self.CurrentTile`)))
  (bind _returnvalue (- (`KismetMathLibrary.Conv_IntToDouble` (`/Game/BLueprints/bp_tileboard.TileSize` (`self.tileBoardRef`))) 1.0))
  (bind _returnvalue_2 (`KismetMathLibrary.FClamp` (+ ActionValue_Y _currenttile_y) 0.0 _returnvalue))
  (bind _returnvalue_3 (`KismetMathLibrary.FClamp` (+ ActionValue_X _currenttile_x) 0.0 _returnvalue))
  ;[1 1 1] Moving
  (:`Started`
    (if (not (`self.DoingShooting`))
      (`SceneComponent.K2_SetRelativeRotation` (`self.StaticMesh`) (`KismetMathLibrary.MakeRotator` 0.0 0.0 (+ (`KismetMathLibrary.SelectFloat` 180.0 0.0 (< ActionValue_X 0.0)) (* ActionValue_Y -90.0))) false false)
      (bind _tile (`/Game/BLueprints/bp_tileboard.FindTile` (`self.tileBoardRef`) (`KismetMathLibrary.MakeVector2D` _returnvalue_3 _returnvalue_2)))
      (if (not (`/Game/BLueprints/BP_Comp_Tile.IsIsland` _tile))
        (bind _output_get (set `self.CurrentTile` (`KismetMathLibrary.MakeVector2D` _returnvalue_3 _returnvalue_2)))
        (bind _tile_2 (`/Game/BLueprints/bp_tileboard.FindTile` (`self.tileBoardRef`) _output_get))
        (`self.K2_SetActorLocation` (`SceneComponent.K2_GetComponentLocation` _tile_2))
        (`self.ActionDone`)))))

(event `Key|SpaceBar`
  (params (Key :type "Key Structure"))
  ;[1 1 1] FireCannon
  (:`Pressed`
    (if (not (`self.DoingShooting`))
      (set `self.DoingShooting` true)
      (for _array_element (`|MakeArray` (`self.Starboard`) (`self.Port`))
        (`|SpawnActorFromClass` "/Game/BLueprints/bp_cannons.bp_cannons_C" (`SceneComponent.K2_GetComponentToWorld` _array_element) "Undefined" "MultiplyWithRoot" null self false null))
      (`KismetSystemLibrary.Delay` 0.75)
      (set `self.DoingShooting` false)
      (`self.ActionDone`))))

(event `ShipDead`
  (bind _returnvalue (`|CreateWidget` "/Game/ui_death.ui_death_C"))
  (`UserWidget.AddToViewport` _returnvalue 0)
  (set `PlayerController.bShowMouseCursor` true (`GameplayStatics.GetPlayerController` 0))
  (`self.K2_DestroyActor`))

(fn `SafePlace`
  (returns (Out :type "Array of /Game/BLueprints/BP_Comp_Tile Object Reference"))
  (locals (SafeTiles :type "Array of /Game/BLueprints/BP_Comp_Tile Object Reference") (extraSafeTiles :type "Array of /Game/BLueprints/BP_Comp_Tile Object Reference"))
  (for _array_element (`self.K2_GetComponentsByClass` (`self.tileBoardRef`) "/Game/BLueprints/BP_Comp_Tile.BP_Comp_Tile_C")
    (if (`/Game/BLueprints/BP_Comp_Tile.IsIsland` _array_element)
      _
      (elif (not (`KismetArrayLibrary.Array_Contains` (`/Game/BLueprints/bp_tileboard.tileWithEnemies` (`self.tileBoardRef`)) _array_element))
        (`KismetArrayLibrary.Array_Add` (`local.extraSafeTiles`) _array_element))))
  (return (`local.extraSafeTiles`)))

(fn `UserConstructionScript`)