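; BP_Cannons is a short-lived cannonball that destroys itself 0.75 seconds after spawning.
; On Sphere3 overlap, the EnemyBall flag selects its valid target.
; An enemy ball calls ShipDead on BP_Character, while a friendly ball destroys BP_EnemyBoats and reports EnemyKilled to its Maker's TileBoardRef.
; The ball destroys itself after either hit and survives overlaps with other actors.
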(event `self.ReceiveBeginPlay`
  (`KismetSystemLibrary.Delay` 0.75)
  (`self.K2_DestroyActor`))

(event `self.Sphere3.OnComponentBeginOverlap`
  (params (OverlappedComponent :type "PrimitiveComponent Object Reference") (OtherActor :type "Actor Object Reference") (OtherComp :type "PrimitiveComponent Object Reference") (OtherBodyIndex :type Integer) (bFromSweep :type Boolean) (SweepResult :type "HitResult Structure (by ref)"))
  (if (`self.EnemyBall`)
    (bind _asbp_character (cast `/Game/BLueprints/BP_Character` OtherActor))
    (`/Game/BLueprints/BP_Character.ShipDead` _asbp_character)
    (`self.K2_DestroyActor`)
    (else
      ;[1 1 1] Good ball
      (bind _asbp_enemy_boats (cast `/Game/Enemies/BP_EnemyBoats` OtherActor))
      (`self.K2_DestroyActor` _asbp_enemy_boats)
      (`/Game/BLueprints/bp_tileboard.EnemyKilled` (`/Game/BLueprints/BP_Character.tileBoardRef` (`self.Maker`)))
      (`self.K2_DestroyActor`))))

(fn `UserConstructionScript`)